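; Player Blueprint that drives the game's startup UI flow and toggles the in-game menu.
; On GameBegin, a GameSave slot leads to a timed Opening widget and then dialogs, while no save shows character selection.
; TaskFinish advances the flow: role selection leads to the story background or, with a save, the opening, and animation completion also leads to the opening.
; Each stage clears MyInstace's loading widget or sets cursor and input mode as needed.
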(event Custom|GameBegin
  (bind _returnvalue (Game|GetPlayerController 0))
  (bind _returnvalue_2 (Game|GetPlayerController 0))
  (bind _returnvalue_3 (SaveGame|DoesSaveGameExist "GameSave"))
  (if _returnvalue_3
    (bind _asmy_instace (Utilities|Casting|CastToMyInstace (Game|GetGameInstance)))
    (Widget|RemovefromParent (Variables|/Game/MyInstace.MyInstace_C|GetLoadingWidget _asmy_instace))
    (bind _returnvalue_4 (UserInterface|CreateWidget "/Game/UI/SceneTip/Opening.Opening_C"))
    (UserInterface|Viewport|AddtoViewport _returnvalue_4 0)
    (Utilities|FlowControl|Delay 5.0)
    (Widget|RemovefromParent _returnvalue_4)
    (bind _returnvalue_5 (UserInterface|CreateWidget "/Game/UI/Dialog/BP_DialogsWidget.BP_DialogsWidget_C" 0 self))
    (Variables|Default|SetDialogWidget _returnvalue_5)
    (bind _asmy_instace_2 (Utilities|Casting|CastToMyInstace (Game|GetGameInstance)))
    (Widget|RemovefromParent (Variables|/Game/MyInstace.MyInstace_C|GetLoadingWidget _asmy_instace_2))
    (UserInterface|Viewport|AddtoViewport _returnvalue_5 0)
    (Variables|/Script/Engine.PlayerController|SetbShowMouseCursor _returnvalue true)
    (Input|SetInputModeGameandUI _returnvalue _returnvalue_5 "DoNotLock" false)
    (else
      (bind _asmy_instace_3 (Utilities|Casting|CastToMyInstace (Game|GetGameInstance)))
      (Widget|RemovefromParent (Variables|/Game/MyInstace.MyInstace_C|GetLoadingWidget _asmy_instace_3))
      (bind _returnvalue_6 (UserInterface|CreateWidget "/Game/UI/CharacterChoose/BP_CharacterWidget.BP_CharacterWidget_C" 0 self))
      (UserInterface|Viewport|AddtoViewport _returnvalue_6 0)
      (Variables|/Script/Engine.PlayerController|SetbShowMouseCursor _returnvalue_2 true)
      (Input|SetInputModeUIOnly _returnvalue_2 _returnvalue_6 "DoNotLock"))))

(event EventTaskFinish
  (params (TaskType :type ETaskType%20Enum :default "NewEnumerator0"))
  (bind _returnvalue (Game|GetPlayerController 0))
  (bind _returnvalue_2 (Game|GetPlayerController 0))
  (switch Utilities|FlowControl|Switch|SwitchonETaskType TaskType
    (:NewEnumerator0
      (bind _returnvalue_3 (UserInterface|CreateWidget "/Game/UI/SceneTip/Opening.Opening_C" :!label _label))
      (UserInterface|Viewport|AddtoViewport _returnvalue_3 0)
      (Utilities|FlowControl|Delay 5.0)
      (Widget|RemovefromParent _returnvalue_3)
      (bind _returnvalue_4 (UserInterface|CreateWidget "/Game/UI/Dialog/BP_DialogsWidget.BP_DialogsWidget_C" 0 self))
      (Variables|Default|SetDialogWidget _returnvalue_4)
      (bind _asmy_instace (Utilities|Casting|CastToMyInstace (Game|GetGameInstance)))
      (Widget|RemovefromParent (Variables|/Game/MyInstace.MyInstace_C|GetLoadingWidget _asmy_instace))
      (UserInterface|Viewport|AddtoViewport _returnvalue_4 0)
      (Variables|/Script/Engine.PlayerController|SetbShowMouseCursor _returnvalue true)
      (Input|SetInputModeGameandUI _returnvalue _returnvalue_4 "DoNotLock" false))
    (:NewEnumerator1
      (bind _returnvalue_5 (SaveGame|DoesSaveGameExist "GameSave"))
      (if _returnvalue_5
        (bind _asmy_instace_2 (Utilities|Casting|CastToMyInstace (Game|GetGameInstance)))
        (Widget|RemovefromParent (Variables|/Game/MyInstace.MyInstace_C|GetLoadingWidget _asmy_instace_2))
        (goto _label)
        (else
          (bind _asmy_instace_3 (Utilities|Casting|CastToMyInstace (Game|GetGameInstance)))
          (Widget|RemovefromParent (Variables|/Game/MyInstace.MyInstace_C|GetLoadingWidget _asmy_instace_3))
          (bind _returnvalue_6 (UserInterface|CreateWidget "/Game/UI/StoryBackground/BP_StoryBackgroundWidget.BP_StoryBackgroundWidget_C" 0 12 self))
          (UserInterface|Viewport|AddtoViewport _returnvalue_6 0)
          (Variables|/Script/Engine.PlayerController|SetbShowMouseCursor _returnvalue_2 true)
          (Input|SetInputModeUIOnly _returnvalue_2 _returnvalue_6 "DoNotLock"))))))

(event Input|ActionEvents|InputActionOpenMenu
  (params (Key :type Key%20Structure :default "None"))
  (bind _returnvalue (Game|GetPlayerController 0))
  (:Pressed
    (bind _ingamemenu (Variables|Default|GetInGameMenu)
      (:then
        (Default|CloseMenu _ingamemenu))
      (:else
        (bind _returnvalue_2 (UserInterface|CreateWidget "/Game/UI/InGameMenu/BP_InGameMenuWidget.BP_InGameMenuWidget_C" 0 self))
        (bind _output_get (Variables|Default|SetInGameMenu _returnvalue_2))
        (UserInterface|Viewport|AddtoViewport _output_get 0)
        (Variables|/Script/Engine.PlayerController|SetbShowMouseCursor _returnvalue true)
        (Input|SetInputModeGameandUI _returnvalue _returnvalue_2 "DoNotLock" false)))))

(fn ConstructionScript)